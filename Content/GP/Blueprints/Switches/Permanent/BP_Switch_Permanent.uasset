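; BP_Switch_Permanent is an interactable switch that toggles the point light of the level's permanent light actor.
; On BeginPlay it caches the first BP_Light_Permanent found via GetActorOfClass, so it is not linked to a specific light instance.
; Its box collision shows a W_PressE prompt widget on overlap and removes it on exit.
; Interact toggles the light's visibility and returns true, while InteractWithBell always returns false.
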(event OnComponentEndOverlap(BoxCollision)
  (params (OverlappedComponent :type Primitive%20Component%20Object%20Reference) (OtherActor :type Actor%20Object%20Reference) (OtherComp :type Primitive%20Component%20Object%20Reference) (OtherBodyIndex :type Integer))
  (Widget|RemovefromParent (Variables|Default|GetInteractWidget)))

(event OnComponentBeginOverlap(BoxCollision)
  (params (OverlappedComponent :type Primitive%20Component%20Object%20Reference) (OtherActor :type Actor%20Object%20Reference) (OtherComp :type Primitive%20Component%20Object%20Reference) (OtherBodyIndex :type Integer) (bFromSweep :type Boolean) (SweepResult :type Hit%20Result%20Structure%20%28by%20ref%29))
  (bind _returnvalue (UserInterface|CreateWidget "/Game/GP/Widgets/W_PressE.W_PressE_C"))
  (bind _output_get (Variables|Default|SetInteractWidget _returnvalue))
  (UserInterface|Viewport|AddtoViewport _output_get 0))

(event EventBeginPlay
  (bind _returnvalue (Actor|GetActorOfClass "/Game/GP/Blueprints/Switches/Permanent/BP_Light_Permanent.BP_Light_Permanent_C"))
  (Variables|Default|SetPermLight _returnvalue))

(fn ConstructionScript)

(fn Interact
  (params (Character :type Character%20Object%20Reference))
  (Rendering|ToggleVisibility (Variables|/Game/GP/Blueprints/Switches/Permanent/BP_Light_Permanent.BP_Light_Permanent_C|GetPointLight (Variables|Default|GetPermLight)) true)
  (return true))

(fn InteractwithBell
  (params (Char :type BPA%20Buttler%20Object%20Reference))
  (return false))