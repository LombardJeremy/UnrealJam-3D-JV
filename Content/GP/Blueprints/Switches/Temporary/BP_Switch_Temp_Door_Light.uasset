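; A temporary interactable switch that turns on a light and opens a set of doors, then reverts after a delay.
; Entering its box shows a press-E widget; Interact lights the level's BP_Light_Temporary and plays a timeline rotating each door.
; Leaving while open removes the widget, waits, then turns off the light and reverses that timeline to close the doors.
; A separate closing timeline is unused, and bell interaction returns false.
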(event OnComponentEndOverlap(BoxCollision)
  (params (OverlappedComponent :type Primitive%20Component%20Object%20Reference) (OtherActor :type Actor%20Object%20Reference) (OtherComp :type Primitive%20Component%20Object%20Reference) (OtherBodyIndex :type Integer))
  (bind _permlight (Variables|Default|GetPermLight))
  (if (Variables|Default|GetisOpen)
    (Widget|RemovefromParent (Variables|Default|GetInteractWidget))
    (Utilities|FlowControl|Delay (Variables|Default|GetLightsOffDuration))
    (if (Variables|/Script/Engine.SceneComponent|GetbVisible (Variables|/Game/GP/Blueprints/Switches/Temporary/BP_Light_Temporary.BP_Light_Temporary_C|GetPointLight _permlight))
      (Rendering|ToggleVisibility (Variables|/Game/GP/Blueprints/Switches/Temporary/BP_Light_Temporary.BP_Light_Temporary_C|GetPointLight _permlight) false)
      (Development|PrintString "Lights off")
      (CallFunction|CECloseDoors))))

(event OnComponentBeginOverlap(BoxCollision)
  (params (OverlappedComponent :type Primitive%20Component%20Object%20Reference) (OtherActor :type Actor%20Object%20Reference) (OtherComp :type Primitive%20Component%20Object%20Reference) (OtherBodyIndex :type Integer) (bFromSweep :type Boolean) (SweepResult :type Hit%20Result%20Structure%20%28by%20ref%29))
  (bind _returnvalue (UserInterface|CreateWidget "/Game/GP/Widgets/W_PressE.W_PressE_C"))
  (bind _output_get (Variables|Default|SetInteractWidget _returnvalue))
  (UserInterface|Viewport|AddtoViewport _output_get 0))

(event Custom|CE_OpenDoor
  (if (not (Variables|Default|GetisOpen))
    ;[1 1 1] Open doors
    (Variables|Default|SetisOpen true)
    (bind _angle (Timeline|T_OpenDoor PlayFromStart)
      (:Update
        (for _array_element (Variables|Default|GetDoors)
          (Transformation|SetActorRotation (.Doors (Utilities|Struct|BreakS_Door _array_element)) (Math|Rotator|Lerp(Rotator) (.InitialRotation (Utilities|Struct|BreakS_Door _array_element)) (.RotationAngle (Utilities|Struct|BreakS_Door _array_element)) _angle))
          (Development|PrintString "doors opened"))))))

(event Custom|CE_CloseDoors
  (if (Variables|Default|GetisOpen)
    ;[1 1 1] Close doors
    (Variables|Default|SetisOpen false)
    ;[1 1 1] Open doors
    (bind _angle (Timeline|T_OpenDoor ReverseFromEnd)
      (:Update
        (for _array_element (Variables|Default|GetDoors)
          (Transformation|SetActorRotation (.Doors (Utilities|Struct|BreakS_Door _array_element)) (Math|Rotator|Lerp(Rotator) (.InitialRotation (Utilities|Struct|BreakS_Door _array_element)) (.RotationAngle (Utilities|Struct|BreakS_Door _array_element)) _angle))
          (Development|PrintString "doors opened"))))))

(event EventBeginPlay
  (bind _returnvalue (Actor|GetActorOfClass "/Game/GP/Blueprints/Switches/Temporary/BP_Light_Temporary.BP_Light_Temporary_C"))
  (Variables|Default|SetPermLight _returnvalue))

(fn ConstructionScript)

(fn Interact
  (params (Character :type Character%20Object%20Reference))
  (Rendering|ToggleVisibility (Variables|/Game/GP/Blueprints/Switches/Temporary/BP_Light_Temporary.BP_Light_Temporary_C|GetPointLight (Variables|Default|GetPermLight)) true)
  (if (Variables|Default|GetisOpen)
    (Development|PrintString "Door is already open !")
    (else
      (CallFunction|CEOpenDoor)
      (return true))))

(fn InteractwithBell
  (params (Char :type BPA%20Buttler%20Object%20Reference))
  (return false))