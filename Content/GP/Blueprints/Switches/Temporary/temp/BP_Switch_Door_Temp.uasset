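; Temporary door switch that swings a set of linked door actors open through interaction or when a BPA_Buttler enters its box.
; Other overlapping actors reveal a press-E widget, and Interact opens the doors unless already open.
; A timeline lerps each door between its initial and target rotation, reversing to close.
; End overlap closes them after the LightsOffDuration delay, hiding the prompt only if open.
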(event OnComponentEndOverlap(BoxCollision)
  (params (OverlappedComponent :type Primitive%20Component%20Object%20Reference) (OtherActor :type Actor%20Object%20Reference) (OtherComp :type Primitive%20Component%20Object%20Reference) (OtherBodyIndex :type Integer))
  (bind _interactwidget (Variables|Default|GetInteractWidget))
  (if (Variables|Default|GetisOpen)
    (Utilities|IsValid _interactwidget
      (:Is%20Valid
        (Variables|/Script/UMG.Widget|SetVisibility _interactwidget "Hidden"))))
  (Utilities|FlowControl|Delay (Variables|Default|GetLightsOffDuration))
  (CallFunction|CECloseDoors))

(event OnComponentBeginOverlap(BoxCollision)
  (params (OverlappedComponent :type Primitive%20Component%20Object%20Reference) (OtherActor :type Actor%20Object%20Reference) (OtherComp :type Primitive%20Component%20Object%20Reference) (OtherBodyIndex :type Integer) (bFromSweep :type Boolean) (SweepResult :type Hit%20Result%20Structure%20%28by%20ref%29))
  (Utilities|Casting|CastToBPA_Buttler OtherActor
    (:then
      (CallFunction|CEOpenDoor))
    (:CastFailed
      (Variables|/Script/UMG.Widget|SetVisibility (Variables|Default|GetInteractWidget) "Visible"))))

(event Custom|CE_OpenDoor
  (if (not (Variables|Default|GetisOpen))
    (Variables|Default|SetisOpen true)
    (bind _angle (Timeline|T_OpenDoor PlayFromStart)
      (:Update
        (for _array_element (Variables|Default|GetDoors)
          (Transformation|SetActorRotation (.Doors (Utilities|Struct|BreakS_Door _array_element)) (Math|Rotator|Lerp(Rotator) (.InitialRotation (Utilities|Struct|BreakS_Door _array_element)) (.RotationAngle (Utilities|Struct|BreakS_Door _array_element)) _angle))
          (Development|PrintString "doors opened"))))))

(event Custom|CE_CloseDoors
  ;[1 1 1] Close doors
  (if (Variables|Default|GetisOpen)
    (Variables|Default|SetisOpen false)
    (bind _angle (Timeline|T_OpenDoor ReverseFromEnd)
      (:Update
        (for _array_element (Variables|Default|GetDoors)
          (Transformation|SetActorRotation (.Doors (Utilities|Struct|BreakS_Door _array_element)) (Math|Rotator|Lerp(Rotator) (.InitialRotation (Utilities|Struct|BreakS_Door _array_element)) (.RotationAngle (Utilities|Struct|BreakS_Door _array_element)) _angle))
          (Development|PrintString "doors opened"))))))

(event EventBeginPlay
  (bind _returnvalue (UserInterface|CreateWidget "/Game/GP/Widgets/W_PressE.W_PressE_C"))
  (bind _output_get (Variables|Default|SetInteractWidget _returnvalue))
  (UserInterface|Viewport|AddtoViewport _output_get 0)
  (Variables|/Script/UMG.Widget|SetVisibility _output_get "Hidden"))

(fn ConstructionScript)

(fn Interact
  (params (Character :type Character%20Object%20Reference))
  (if (Variables|Default|GetisOpen)
    (Development|PrintString "Door is already open !")
    (else
      (CallFunction|CEOpenDoor)
      (return true))))

(fn InteractwithBell
  (params (Char :type BPA%20Buttler%20Object%20Reference))
  (return false))