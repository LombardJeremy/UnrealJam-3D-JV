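; Temporary switch that opens a set of doors and controls linked lights and lamps through a trigger box or interaction.
; Butler overlap sends it to an interact point, opens doors and turns lights on; other actors get a press-E widget.
; Interact toggles only the linked lights and opens doors; ending overlap closes and darkens everything, optionally after a delay.
; One timeline lerps door rotations and reverses to close, leaving the separate close timeline unused.
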(event OnComponentEndOverlap(BoxCollision)
  (params (OverlappedComponent :type Primitive%20Component%20Object%20Reference) (OtherActor :type Actor%20Object%20Reference) (OtherComp :type Primitive%20Component%20Object%20Reference) (OtherBodyIndex :type Integer))
  (bind _lights (Variables|Default|GetLIGHTS))
  (bind _lampadere (Variables|Default|GetLAMPADERE))
  (Utilities|IsValid 0
    (:Is%20Valid
      (Widget|RemovefromParent (Variables|Default|GetInteractWidget)))
    (:Is%20Not%20Valid
      _))
  (if (Variables|Default|GetisOpen)
    (if (Variables|Default|GetIsChrono)
      (Utilities|FlowControl|Delay (Variables|Default|GetLightsOffDuration)))
    (CallFunction|CECloseDoors)
    (if (Utilities|Array|IsEmpty _lights)
      _
      (else
        (for _array_element _lights
          (if (Rendering|IsVisible (Variables|/Script/Engine.Light|GetLightComponent _array_element))
            (Rendering|SetVisibility (Variables|/Script/Engine.Light|GetLightComponent _array_element) false true)))))
    (if (not (Utilities|Array|IsEmpty _lampadere))
      (for _array_element_2 _lampadere
        (Utilities|IsValid _array_element_2
          (:Is%20Valid
            (bind _aslight_component (Utilities|Casting|CastToLightComponent (Components|GetChildComponent (Variables|/Game/GA/Props/arnaud_light.arnaud_light_C|GetLustre_lustre _array_element_2) 0)))
            (if (Rendering|IsVisible _aslight_component)
              (Rendering|SetVisibility _aslight_component false true)))))
      (Development|PrintString "Lights off"))))

(event OnComponentBeginOverlap(BoxCollision)
  (params (OverlappedComponent :type Primitive%20Component%20Object%20Reference) (OtherActor :type Actor%20Object%20Reference) (OtherComp :type Primitive%20Component%20Object%20Reference) (OtherBodyIndex :type Integer) (bFromSweep :type Boolean) (SweepResult :type Hit%20Result%20Structure%20%28by%20ref%29))
  (bind _lights (Variables|Default|GetLIGHTS))
  (bind _lampadere (Variables|Default|GetLAMPADERE))
  (bind _point_for_butler (Variables|Default|GetPoint%20for%20butler))
  (bind _asbpa_buttler (Utilities|Casting|CastToBPA_Buttler OtherActor)
    (:then
      (Default|GotoTargetInteract _asbpa_buttler (Transformation|GetWorldLocation _point_for_butler) (Transformation|GetWorldRotation _point_for_butler))
      (CallFunction|CEOpenDoor)
      (if (Utilities|Array|IsEmpty _lights)
        _
        (else
          (for _array_element _lights
            (Utilities|IsValid (Variables|/Script/Engine.Light|GetLightComponent _array_element)
              (:Is%20Valid
                (Rendering|SetVisibility (Variables|/Script/Engine.Light|GetLightComponent _array_element) true true))))))
      (if (not (Utilities|Array|IsEmpty _lampadere))
        (for _array_element_2 _lampadere
          (Utilities|IsValid _array_element_2
            (:Is%20Valid
              (bind _aslight_component (Utilities|Casting|CastToLightComponent (Components|GetChildComponent (Variables|/Game/GA/Props/arnaud_light.arnaud_light_C|GetLustre_lustre _array_element_2) 0)))
              (Rendering|SetVisibility _aslight_component true true))))))
    (:CastFailed
      (bind _returnvalue (UserInterface|CreateWidget "/Game/GP/Widgets/W_PressE.W_PressE_C"))
      (bind _output_get (Variables|Default|SetInteractWidget _returnvalue))
      (UserInterface|Viewport|AddtoViewport _output_get 0))))

(event Custom|CE_OpenDoor
  (if (not (Variables|Default|GetisOpen))
    ;[1 1 1] Open doors
    (Variables|Default|SetisOpen true)
    (bind _angle (Timeline|T_OpenDoor PlayFromStart)
      (:Update
        (for _array_element (Variables|Default|GetDoors)
          (Transformation|SetActorRotation (.Doors (Utilities|Struct|BreakS_Door _array_element)) (Math|Rotator|Lerp(Rotator) (.InitialRotation (Utilities|Struct|BreakS_Door _array_element)) (.RotationAngle (Utilities|Struct|BreakS_Door _array_element)) _angle))
          (Development|PrintString "doors opened"))))))

(event Custom|CE_CloseDoors
  (if (Variables|Default|GetisOpen)
    ;[1 1 1] Close doors
    (Variables|Default|SetisOpen false)
    ;[1 1 1] Open doors
    (bind _angle (Timeline|T_OpenDoor ReverseFromEnd)
      (:Update
        (for _array_element (Variables|Default|GetDoors)
          (Transformation|SetActorRotation (.Doors (Utilities|Struct|BreakS_Door _array_element)) (Math|Rotator|Lerp(Rotator) (.InitialRotation (Utilities|Struct|BreakS_Door _array_element)) (.RotationAngle (Utilities|Struct|BreakS_Door _array_element)) _angle))
          (Development|PrintString "doors opened"))))))

(fn ConstructionScript)

(fn Interact
  (params (Character :type Character%20Object%20Reference))
  (for _array_element (Variables|Default|GetLIGHTS)
    (Rendering|ToggleVisibility (Variables|/Script/Engine.Light|GetLightComponent _array_element) true))
  (if (Variables|Default|GetisOpen)
    (Development|PrintString "Door is already open !")
    (else
      (CallFunction|CEOpenDoor)
      (return true))))

(fn InteractwithBell
  (params (Char :type BPA%20Buttler%20Object%20Reference))
  (return false))