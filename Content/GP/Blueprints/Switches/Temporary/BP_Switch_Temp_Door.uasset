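; BP_Switch_Temp_Door is an interactable switch that temporarily opens an array of doors.
; Entering its box shows a press-E widget, and Interact plays a timeline that lerps each door to its target rotation unless already open.
; Leaving the box removes the widget and, after LightsOffDuration, always plays the closing timeline.
; A BP_Light_Temporary reference is cached on BeginPlay but unused, and bell interaction returns false.
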(event OnComponentEndOverlap(BoxCollision)
  (params (OverlappedComponent :type Primitive%20Component%20Object%20Reference) (OtherActor :type Actor%20Object%20Reference) (OtherComp :type Primitive%20Component%20Object%20Reference) (OtherBodyIndex :type Integer))
  (Widget|RemovefromParent (Variables|Default|GetInteractWidget))
  (Utilities|FlowControl|Delay (Variables|Default|GetLightsOffDuration))
  (Development|PrintString "Lights off")
  (CallFunction|CECloseDoors))

(event OnComponentBeginOverlap(BoxCollision)
  (params (OverlappedComponent :type Primitive%20Component%20Object%20Reference) (OtherActor :type Actor%20Object%20Reference) (OtherComp :type Primitive%20Component%20Object%20Reference) (OtherBodyIndex :type Integer) (bFromSweep :type Boolean) (SweepResult :type Hit%20Result%20Structure%20%28by%20ref%29))
  (bind _returnvalue (UserInterface|CreateWidget "/Game/GP/Widgets/W_PressE.W_PressE_C"))
  (bind _output_get (Variables|Default|SetInteractWidget _returnvalue))
  (UserInterface|Viewport|AddtoViewport _output_get 0))

(event Custom|CE_OpenDoor
  ;[1 1 1] Open doors
  (bind _angle (Timeline|T_OpenDoor PlayFromStart)
    (:Update
      (for _array_element (Variables|Default|GetDoors)
        (Transformation|SetActorRotation (.Doors (Utilities|Struct|BreakS_Door _array_element)) (Math|Rotator|Lerp(Rotator) (.InitialRotation (Utilities|Struct|BreakS_Door _array_element)) (.RotationAngle (Utilities|Struct|BreakS_Door _array_element)) _angle))
        (Variables|Default|SetisOpen true)
        (Development|PrintString "doors opened")))))

(event Custom|CE_CloseDoors
  ;[1 1 1] Close doors
  (bind _rotation (Timeline|T_CloseDoor PlayFromStart)
    (:Update
      (for _array_element (Variables|Default|GetDoors)
        (Transformation|SetActorRotation (.Doors (Utilities|Struct|BreakS_Door _array_element)) (Math|Rotator|Lerp(Rotator) (.RotationAngle (Utilities|Struct|BreakS_Door _array_element)) (.InitialRotation (Utilities|Struct|BreakS_Door _array_element)) _rotation))
        (Variables|Default|SetisOpen false)
        (Development|PrintString "doors closed")))))

(event EventBeginPlay
  (bind _returnvalue (Actor|GetActorOfClass "/Game/GP/Blueprints/Switches/Temporary/BP_Light_Temporary.BP_Light_Temporary_C"))
  (Variables|Default|SetPermLight _returnvalue))

(fn ConstructionScript)

(fn Interact
  (params (Character :type Character%20Object%20Reference))
  (if (Variables|Default|GetisOpen)
    (Development|PrintString "Door is already open !")
    (else
      (CallFunction|CEOpenDoor)
      (return true))))

(fn InteractwithBell
  (params (Char :type BPA%20Buttler%20Object%20Reference))
  (return false))