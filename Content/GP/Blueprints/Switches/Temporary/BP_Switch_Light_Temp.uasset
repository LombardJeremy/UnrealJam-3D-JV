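; Temporary switch actor that turns a set of lights on and off and tracks an open/closed door state.
; Overlap sends the butler to an interact point, lights up and opens; other actors get a press-E widget, and Interact toggles the lights.
; Leaving while open removes the widget, optionally waits, then closes and switches lights off.
; Door rotation timelines are disconnected, so opening and closing only set IsOpen.
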(event OnComponentEndOverlap(BoxCollision)
  (params (OverlappedComponent :type Primitive%20Component%20Object%20Reference) (OtherActor :type Actor%20Object%20Reference) (OtherComp :type Primitive%20Component%20Object%20Reference) (OtherBodyIndex :type Integer))
  (bind _interactwidget (Variables|Default|GetInteractWidget))
  (if (Variables|Default|GetisOpen)
    (Utilities|IsValid _interactwidget
      (:Is%20Valid
        (Widget|RemovefromParent _interactwidget))
      (:Is%20Not%20Valid
        _))
    (if (Variables|Default|GetIsChrono)
      (Utilities|FlowControl|Delay (Variables|Default|GetLightsOffDuration)))
    (CallFunction|CECloseDoors)
    (for _array_element (Variables|Default|GetLIGHTS)
      (if (Rendering|IsVisible (Variables|/Script/Engine.Light|GetLightComponent _array_element))
        (Rendering|SetVisibility (Variables|/Script/Engine.Light|GetLightComponent _array_element) false true)))
    (Development|PrintString "Lights off")))

(event OnComponentBeginOverlap(BoxCollision)
  (params (OverlappedComponent :type Primitive%20Component%20Object%20Reference) (OtherActor :type Actor%20Object%20Reference) (OtherComp :type Primitive%20Component%20Object%20Reference) (OtherBodyIndex :type Integer) (bFromSweep :type Boolean) (SweepResult :type Hit%20Result%20Structure%20%28by%20ref%29))
  (bind _point_for_butler (Variables|Default|GetPoint%20for%20butler))
  (bind _asbpa_buttler (Utilities|Casting|CastToBPA_Buttler OtherActor)
    (:then
      (Default|GotoTargetInteract _asbpa_buttler (Transformation|GetWorldLocation _point_for_butler) (Transformation|GetWorldRotation _point_for_butler))
      (CallFunction|CEOpenDoor)
      (for _array_element (Variables|Default|GetLIGHTS)
        (Rendering|SetVisibility (Variables|/Script/Engine.Light|GetLightComponent _array_element) true true)))
    (:CastFailed
      (bind _returnvalue (UserInterface|CreateWidget "/Game/GP/Widgets/W_PressE.W_PressE_C"))
      (bind _output_get (Variables|Default|SetInteractWidget _returnvalue))
      (UserInterface|Viewport|AddtoViewport _output_get 0))))

(event Custom|CE_OpenDoor
  (if (not (Variables|Default|GetisOpen))
    ;[1 1 1] Open doors
    (Variables|Default|SetisOpen true)))

(event Custom|CE_CloseDoors
  (if (Variables|Default|GetisOpen)
    ;[1 1 1] Close doors
    (Variables|Default|SetisOpen false)))

(fn ConstructionScript)

(fn Interact
  (params (Character :type Character%20Object%20Reference))
  (for _array_element (Variables|Default|GetLIGHTS)
    (Rendering|ToggleVisibility (Variables|/Script/Engine.Light|GetLightComponent _array_element) true))
  (if (Variables|Default|GetisOpen)
    (Development|PrintString "Door is already open !")
    (else
      (CallFunction|CEOpenDoor)
      (return true))))

(fn InteractwithBell
  (params (Char :type BPA%20Buttler%20Object%20Reference))
  (return false))