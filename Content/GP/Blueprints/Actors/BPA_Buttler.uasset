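; Butler character Blueprint that walks to given locations via AI movement, with animations driven directly by montages.
; It starts a walk montage on BeginPlay and whenever either move event issues AIMoveTo.
; GoToTarget switches to idle on arrival, while GoToTargetInteract snaps to a supplied rotation and plays an interact montage, then a loop montage after a fixed delay.
; Failed moves only print a debug message.
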(event Custom|Go%20To%20Target
  (params (Target%20Loc :type Vector))
  (AI|AIMoveTo self Target%20Loc 0 5.0 false
    (:then
      (Animation|PlayAnimMontage "/Game/GA/Props/Butler/NEW/ANIMATION/Walk_Anim.Walk_Anim" 1.0 "None"))
    (:OnSuccess
      (Development|PrintString "SUCESS")
      (Animation|PlayAnimMontage "/Game/GA/Props/Butler/NEW/ANIMATION/Idle_Anim.Idle_Anim" 1.0 "None"))
    (:OnFail
      (Development|PrintString "FAILED"))))

(event Custom|Go%20To%20Target%20Interact
  (params (Target%20Loc :type Vector) (Rotation :type Rotator))
  (bind _self self)
  (AI|AIMoveTo _self Target%20Loc 0 5.0 false
    (:then
      (Animation|PlayAnimMontage "/Game/GA/Props/Butler/NEW/ANIMATION/Walk_Anim.Walk_Anim" 1.0 "None"))
    (:OnSuccess
      (Development|PrintString "SUCESS")
      (Transformation|SetActorRotation _self Rotation)
      (Animation|PlayAnimMontage "/Game/GA/Props/Butler/NEW/ANIMATION/Interact_Anim.Interact_Anim" 1.0 "None")
      (Utilities|FlowControl|Delay 1.6)
      (Animation|PlayAnimMontage "/Game/GA/Props/Butler/NEW/ANIMATION/InteractLoop_Anim.InteractLoop_Anim" 1.0 "None"))
    (:OnFail
      (Development|PrintString "FAILED"))))

(event EventBeginPlay
  (Animation|PlayAnimMontage "/Game/GA/Props/Butler/NEW/ANIMATION/Walk_Anim.Walk_Anim" 1.0 "None"))

(fn ConstructionScript)