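; BP_WallLevier is an interactable lever that rotates a configured set of walls when pulled.
; Interact starts two timelines at once: one pitches the handle, the other lerps each WallRotations actor toward its target rotation.
; The lerp starts from each wall's current rotation on every update, so easing compounds.
; Bell interaction returns false, and the BP_Door cached at BeginPlay is unused here.
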(event Custom|CE_PullHandle
  ;[1 1 1] Activate lever to rotate walls
  (bind _angle (Timeline|PullHandle Play)
    (:Update
      (Transformation|SetRelativeRotation (Variables|Default|GetOffsetHandle) (Math|Rotator|MakeRotator 0.0 _angle 0.0) false false))))

(event Custom|CE_RotateWalls
  ;[1 1 1] Rotate walls
  (bind _angle (Timeline|RotateWalls Play)
    (:Update
      (for _array_element (Variables|Default|GetWallRotations)
        (Transformation|SetActorRotation (.Walls (Utilities|Struct|BreakS_Wall _array_element)) (Math|Rotator|Lerp(Rotator) (Transformation|GetActorRotation (.Walls (Utilities|Struct|BreakS_Wall _array_element))) (.RotationAngle (Utilities|Struct|BreakS_Wall _array_element)) _angle))))))

(event EventBeginPlay
  (bind _returnvalue (Actor|GetActorOfClass "/Game/GP/Blueprints/BP_Door.BP_Door_C"))
  (Variables|Default|SetDoor _returnvalue))

(fn ConstructionScript)

(fn Interact
  (params (Character :type Character%20Object%20Reference))
  (CallFunction|CEPullHandle)
  (CallFunction|CERotateWalls)
  (return true))

(fn InteractwithBell
  (params (Char :type BPA%20Buttler%20Object%20Reference))
  (return false))